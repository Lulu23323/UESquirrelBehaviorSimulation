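; Niagara actor for a squirrel crowd effect that is kept aware of the player's position.
; Every Tick it writes the player character's location into the system's User.PlayerLocation parameter.
; Pressing Q fires a debug-drawn Camera-channel line trace from the player along the follow camera's forward direction, but the hit result is unused.
; A Niagara array position read is left unconnected.
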(event Custom|Press%20Q
  (bind _returnvalue (Game|GetPlayerCharacter 0))
  (bind _returnvalue_2 (Transformation|GetActorLocation _returnvalue))
  ;[0.15 0.15 0.15 0.5] Shoot Line Trace
  (bind _asbp_third_person_character (Utilities|Casting|CastToBP_ThirdPersonCharacter (Game|Player|GetPlayerPawn 0)))
  (bind _outhit (Collision|LineTraceByChannel _returnvalue_2 (+ _returnvalue_2 (* (Math|Vector|GetForwardVector (Transformation|GetWorldRotation (Variables|/Game/ThirdPerson/Blueprints/BP_ThirdPersonCharacter.BP_ThirdPersonCharacter_C|GetFollowCamera _asbp_third_person_character))) (Math|Conversions|ToVector(Float) 1.5e+04))) "TraceTypeQuery2" false 0 "ForDuration" true "(R=1.000000,G=0.000000,B=0.000000,A=1.000000)" "(R=0.000000,G=1.000000,B=0.000000,A=1.000000)" 2.0)))

(event EventBeginPlay)

(event EventTick
  (params (DeltaSeconds :type Float%20%28single-precision%29))
  ;[0.15 0.15 0.15 0.5] Update Player location to Squirrel system
  (Niagara|SetNiagaraVariable(Vector3) (Variables|Default|GetNiagaraComponent1) "User.PlayerLocation" (Transformation|GetActorLocation (Game|GetPlayerCharacter 0))))

(fn ConstructionScript)